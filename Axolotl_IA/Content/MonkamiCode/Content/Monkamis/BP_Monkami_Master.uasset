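; Base Monkami creature Blueprint handling health, attacking, death and a clickable tactical menu.
; BeginPlay randomizes Speed, plays a sound and fills the health bar widget with nickname and health.
; Damage updates the bar and triggers Death once, which, only under a wild Monkami AI controller, stops AI logic, plays montage and sound, then destroys the actor.
; Attack plays a montage while alive, and clicking the mesh calls the tactical menu's visibility toggle.
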(event OnClicked(Mesh)
  (params (TouchedComponent :type Primitive%20Component%20Object%20Reference) (ButtonPressed :type Key%20Structure :default "None"))
  (Rendering|ToggleVisibility (Variables|Default|GetMenuTactico) false))

(event Custom|Death
  ;[1 1 1] Muerte
  (bind _asaicontroller (Utilities|Casting|CastToAIController (Pawn|GetController)))
  (bind _asaic_monkami_wild (Utilities|Casting|CastToAIC_Monkami_Wild _asaicontroller))
  (AI|Logic|StopLogic (Variables|/Script/AIModule.AIController|GetBrainComponent _asaic_monkami_wild) "Death")
  (Animation|PlayAnimMontage 0 1.0 "None")
  (Audio|PlaySoundatLocation 0 "0, 0, 0" "0, 0, 0" 1.0 1.0 0.0 0 0 0 0)
  (Utilities|FlowControl|Delay 3.0)
  (Actor|DestroyActor))

(event Custom|Attack
  ;[1 1 1] Atacar
  (if (not (Variables|Default|GetIsDead))
    (Animation|PlayAnimMontage 0 1.0 "None")))

(event EventBeginPlay
  (Variables|Default|SetSpeed (Math|Random|RandomFloatinRange 1e+01 1e+02))
  (bind _aswbp_health_bar (Utilities|Casting|CastToWBP_HealthBar (UserInterface|GetUserWidgetObject (Variables|Default|GetHealthBarWidget))))
  ;[1 0.1759 0.7377] Variables de nacimiento
  (Variables|Default|SetMonsterID (Variables|Default|GetMonsterID))
  (Variables|Default|SetTeamID (Variables|Default|GetTeamID))
  (Variables|Default|SetWild (Variables|Default|GetWild))
  (Variables|/Script/UMG.TextBlock|SetText (Variables|/Game/MonkamiCode/Content/Monkamis/WBP_HealthBar.WBP_HealthBar_C|GetTxt_Name _aswbp_health_bar) (Variables|Default|GetMonsterNickname))
  (Variables|Default|SetForSpawn (Variables|Default|GetForSpawn))
  (Variables|Default|SetHabilities (Variables|Default|GetHabilities))
  (Progress|SetPercent (Variables|/Game/MonkamiCode/Content/Monkamis/WBP_HealthBar.WBP_HealthBar_C|GetBar_Health _aswbp_health_bar) (/ (Variables|Default|GetCurrentHealth) (Variables|Default|GetMaxHealth)))
  (Variables|Default|SetMyHealthBarRef (Variables|/Game/MonkamiCode/Content/Monkamis/WBP_HealthBar.WBP_HealthBar_C|GetBar_Health _aswbp_health_bar))
  (Audio|PlaySoundatLocation 0 "0, 0, 0" "0, 0, 0" 1.0 1.0 0.0 0 0 0 0))

(event Collision|EventActorBeginOverlap
  (params (OtherActor :type Actor%20Object%20Reference)))

(event EventTick
  (params (DeltaSeconds :type Float%20%28single-precision%29)))

(event Game|Damage|EventAnyDamage
  (params (Damage :type Float%20%28single-precision%29) (DamageType :type Damage%20Type%20Object%20Reference) (InstigatedBy :type Controller%20Object%20Reference) (DamageCauser :type Actor%20Object%20Reference))
  ;[1 1 1] Recivir daño
  (Variables|Default|SetCurrentHealth (- (Variables|Default|GetCurrentHealth) Damage))
  (Audio|PlaySoundatLocation 0 "0, 0, 0" "0, 0, 0" 1.0 1.0 0.0 0 0 0 0)
  (Progress|SetPercent (Variables|Default|GetMyHealthBarRef) (/ (Variables|Default|GetCurrentHealth) (Variables|Default|GetMaxHealth)))
  (if (and (<= (Variables|Default|GetCurrentHealth) 0.0) (not (Variables|Default|GetIsDead)))
    (Variables|Default|SetIsDead true)
    (CallFunction|Death)))

(fn ConstructionScript)
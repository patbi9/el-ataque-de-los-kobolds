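; BP_Spell_Explosion is a card spell actor that deals explosion damage to a single target.
; When ExecuteSpell runs, it spawns an emitter at the target's location, applies a fixed amount of damage to that target, then destroys itself.
; BeginPlay, overlap and Tick events are disabled stubs, so all behaviour lives in that one event.
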(event EventBeginPlay
  (|CallParentFunction) ; This node is disabled and will not be called.\nDrag off pins to build functionality.
)

(event Collision|EventActorBeginOverlap
  (params (OtherActor :type Actor%20Object%20Reference))
  (|CallParentFunction OtherActor) ; This node is disabled and will not be called.\nDrag off pins to build functionality.
)

(event EventTick
  (params (DeltaSeconds :type Float%20%28single-precision%29))
  (|CallParentFunction DeltaSeconds) ; This node is disabled and will not be called.\nDrag off pins to build functionality.
)

(event EventExecuteSpell
  (params (Target :type BP%20Monkami%20Master%20Object%20Reference) (Caster :type BP%20Monkami%20Master%20Object%20Reference))
  (Effects|SpawnEmitteratLocation 0 (Transformation|GetActorLocation Target))
  (Game|Damage|ApplyDamage Target 4e+01 0 0)
  (Actor|DestroyActor))

(fn ConstructionScript
  (|CallParentFunction))
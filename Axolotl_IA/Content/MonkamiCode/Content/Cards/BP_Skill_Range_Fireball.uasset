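; BP_Skill_Range_Fireball is a card skill Blueprint for a ranged fireball spell.
; On ExecuteSpell it spawns a BP_Projectile_HomingMaster at the caster's transform, passing the caster as instigator and MyCaster along with the effect value.
; It then sets the projectile movement's homing target to the target's root component, leaving the rest to the projectile.
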(event EventBeginPlay
  (|CallParentFunction) ; This node is disabled and will not be called.\nDrag off pins to build functionality.
)

(event Collision|EventActorBeginOverlap
  (params (OtherActor :type Actor%20Object%20Reference))
  (|CallParentFunction OtherActor) ; This node is disabled and will not be called.\nDrag off pins to build functionality.
)

(event EventTick
  (params (DeltaSeconds :type Float%20%28single-precision%29))
  (|CallParentFunction DeltaSeconds) ; This node is disabled and will not be called.\nDrag off pins to build functionality.
)

(event EventExecuteSpell
  (params (Target :type BP%20Monkami%20Master%20Object%20Reference) (Caster :type BP%20Monkami%20Master%20Object%20Reference) (EffectValue :type Float%20%28double-precision%29))
  (bind _returnvalue (Game|SpawnActorfromClass "/Game/BP_Projectile_HomingMaster.BP_Projectile_HomingMaster_C" (Transformation|GetActorTransform Caster) "Undefined" "MultiplyWithRoot" 0 Caster EffectValue Caster))
  (Variables|/Script/Engine.ProjectileMovementComponent|SetHomingTargetComponent (Variables|/Game/BP_Projectile_HomingMaster.BP_Projectile_HomingMaster_C|GetProjectileMovement _returnvalue) (Variables|/Script/Engine.Actor|GetRootComponent Target)))

(fn ConstructionScript
  (|CallParentFunction))
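; BP_Skill_SelfHeal is a card skill that heals the Monkami that casts it.
; ExecuteSpell casts the caster to BP_Monkami_Master, adds the effect value to its current health and clamps the result between zero and max health.
; It then sets the caster's health bar directly to the new health ratio, with no other active event logic.
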(event EventBeginPlay
  (|CallParentFunction) ; This node is disabled and will not be called.\nDrag off pins to build functionality.
)

(event Collision|EventActorBeginOverlap
  (params (OtherActor :type Actor%20Object%20Reference))
  (|CallParentFunction OtherActor) ; This node is disabled and will not be called.\nDrag off pins to build functionality.
)

(event EventTick
  (params (DeltaSeconds :type Float%20%28single-precision%29))
  (|CallParentFunction DeltaSeconds) ; This node is disabled and will not be called.\nDrag off pins to build functionality.
)

(event EventExecuteSpell
  (params (Target :type BP%20Monkami%20Master%20Object%20Reference) (Caster :type BP%20Monkami%20Master%20Object%20Reference) (EffectValue :type Float%20%28double-precision%29))
  (bind _asbp_monkami_master (Utilities|Casting|CastToBP_Monkami_Master Caster))
  (bind _output_get (Variables|/Game/Monkamis/BP_Monkami_Master.BP_Monkami_Master_C|SetCurrentHealth _asbp_monkami_master (Math|Float|Clamp(Float) (+ (Variables|/Game/Monkamis/BP_Monkami_Master.BP_Monkami_Master_C|GetCurrentHealth _asbp_monkami_master) EffectValue) 0.0 (Variables|/Game/Monkamis/BP_Monkami_Master.BP_Monkami_Master_C|GetMaxHealth _asbp_monkami_master))))
  (Progress|SetPercent (Variables|/Game/Monkamis/BP_Monkami_Master.BP_Monkami_Master_C|GetMyHealthBarRef _asbp_monkami_master) (/ _output_get (Variables|/Game/Monkamis/BP_Monkami_Master.BP_Monkami_Master_C|GetMaxHealth _asbp_monkami_master))))

(fn ConstructionScript
  (|CallParentFunction))
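; BP_Skill_SpawnTerrain is a card skill actor that spawns a terrain piece for a Monkami caster.
; On ExecuteSpell it casts the caster to BP_Monkami_Master and spawns a BP_Terrain at that caster's ForSpawn transform, passing ForSpawn as the new terrain's parent tile (CasillaPadre).
; The skill actor then destroys itself, and does nothing if the cast fails.
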(event EventBeginPlay
  (|CallParentFunction) ; This node is disabled and will not be called.\nDrag off pins to build functionality.
)

(event Collision|EventActorBeginOverlap
  (params (OtherActor :type Actor%20Object%20Reference))
  (|CallParentFunction OtherActor) ; This node is disabled and will not be called.\nDrag off pins to build functionality.
)

(event EventTick
  (params (DeltaSeconds :type Float%20%28single-precision%29))
  (|CallParentFunction DeltaSeconds) ; This node is disabled and will not be called.\nDrag off pins to build functionality.
)

(event EventExecuteSpell
  (params (Target :type BP%20Monkami%20Master%20Object%20Reference) (Caster :type BP%20Monkami%20Master%20Object%20Reference) (EffectValue :type Float%20%28double-precision%29))
  (bind _asbp_monkami_master (Utilities|Casting|CastToBP_Monkami_Master Caster))
  (Game|SpawnActorfromClass "/Game/BP_Terrain.BP_Terrain_C" (Transformation|GetActorTransform (Variables|/Game/Monkamis/BP_Monkami_Master.BP_Monkami_Master_C|GetForSpawn _asbp_monkami_master)) "Undefined" "MultiplyWithRoot" 0 (Variables|/Game/Monkamis/BP_Monkami_Master.BP_Monkami_Master_C|GetForSpawn _asbp_monkami_master) 0)
  (Actor|DestroyActor))

(fn ConstructionScript
  (|CallParentFunction))
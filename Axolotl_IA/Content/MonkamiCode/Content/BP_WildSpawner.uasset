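; BP_WildSpawner spawns wild Monkamis on detected or placed BP_ARFloor actors in the AR world.
; Tick runs through a SpawnRate Delay and spawns while MaxWildMonkamis, a counter that only increments here, is below two.
; Spawning looks up the first MyCardTable row name in DT_Monkamis for class and stats.
; Location comes from random reachable-point queries sized by floor bounds, raised slightly in Z.
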(event Custom|SpawnWildMonkami
  ;[1 1 1] Spawn
  (bind _outactors (Actor|GetAllActorsOfClass "/Game/BP_ARFloor.BP_ARFloor_C"))
  (if (> (Utilities|Array|Length _outactors) 0)
    (bind _outrownames (DataTable|GetDataTableRowNames (Variables|Default|GetMyCardTable)))
    (bind _returnvalue (Utilities|GetDataTableRow "/Game/Monkamis/DT_Monkamis.DT_Monkamis" (Utilities|Array|Get(acopy) _outrownames))
      (:then
        (if (.ReturnValue (AI|Navigation|GetRandomReachablePointinRadius (Transformation|GetActorLocation (Utilities|Array|Get(acopy) _outactors (Math|Random|RandomIntegerinRange 0 (- (Utilities|Array|Length _outactors) 1)))) (Math|Vector|VectorLength (.BoxExtent (Collision|GetActorBounds (Utilities|Array|Get(acopy) _outactors (Math|Random|RandomIntegerinRange 0 (- (Utilities|Array|Length _outactors) 1))) true false))) 0 0))
          (Game|SpawnActorfromClass (.MonsterClass (Utilities|Struct|BreakST_MonkamiData _returnvalue)) (Math|Transform|MakeTransform (Math|Vector|MakeVector (.X (Math|Vector|BreakVector (.RandomLocation (AI|Navigation|GetRandomReachablePointinRadius (Transformation|GetActorLocation (Utilities|Array|Get(acopy) _outactors (Math|Random|RandomIntegerinRange 0 (- (Utilities|Array|Length _outactors) 1)))) (Math|Vector|VectorLength (.BoxExtent (Collision|GetActorBounds (Utilities|Array|Get(acopy) _outactors (Math|Random|RandomIntegerinRange 0 (- (Utilities|Array|Length _outactors) 1))) true false))) 0 0)))) (.Y (Math|Vector|BreakVector (.RandomLocation (AI|Navigation|GetRandomReachablePointinRadius (Transformation|GetActorLocation (Utilities|Array|Get(acopy) _outactors (Math|Random|RandomIntegerinRange 0 (- (Utilities|Array|Length _outactors) 1)))) (Math|Vector|VectorLength (.BoxExtent (Collision|GetActorBounds (Utilities|Array|Get(acopy) _outactors (Math|Random|RandomIntegerinRange 0 (- (Utilities|Array|Length _outactors) 1))) true false))) 0 0)))) (+ (.Z (Math|Vector|BreakVector (.RandomLocation (AI|Navigation|GetRandomReachablePointinRadius (Transformation|GetActorLocation (Utilities|Array|Get(acopy) _outactors (Math|Random|RandomIntegerinRange 0 (- (Utilities|Array|Length _outactors) 1)))) (Math|Vector|VectorLength (.BoxExtent (Collision|GetActorBounds (Utilities|Array|Get(acopy) _outactors (Math|Random|RandomIntegerinRange 0 (- (Utilities|Array|Length _outactors) 1))) true false))) 0 0)))) 1e+01))) "Undefined" "MultiplyWithRoot" 0 0 (.DisplayName (Utilities|Struct|BreakST_MonkamiData _returnvalue)) true (.ID (Utilities|Struct|BreakST_MonkamiData _returnvalue)) 0 (.ListaDeHabilidades (Utilities|Struct|BreakST_MonkamiData _returnvalue)) 0)
          (bind _result (Math|Integer|IncrementInt (Variables|Default|GetMaxWildMonkamis))
            (:%20%20
              (Variables|Default|SetMaxWildMonkamis _result))))))))

(event EventBeginPlay)

(event Collision|EventActorBeginOverlap
  (params (OtherActor :type Actor%20Object%20Reference)))

(event EventTick
  (params (DeltaSeconds :type Float%20%28single-precision%29))
  (Utilities|FlowControl|Delay (Variables|Default|GetSpawnRate))
  (if (< (Variables|Default|GetMaxWildMonkamis) 2)
    (CallFunction|SpawnWildMonkami)))

(fn ConstructionScript)